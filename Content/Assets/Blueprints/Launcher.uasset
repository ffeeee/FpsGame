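; Launcher weapon Blueprint that fires one projectile per Fire call.
; Fire calls ShootOnce, which uses the time since the last shot against ShootAniTime to limit the fire rate.
; An allowed shot spawns a Bullet at the Mazzle component's transform, plays a launcher montage on GunOwner and records the shot time.
; StopFire is empty, so there is no held or automatic fire logic here.
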(event EventBeginPlay)

(event Collision|EventActorBeginOverlap
  (params (OtherActor :type Actor%20Object%20Reference)))

(event EventTick
  (params (DeltaSeconds :type Float%20%28single-precision%29)))

(event EventFire
  (Utilities|FlowControl|Sequence
    (:then_0
      (CallFunction|ShootOnce))))

(event EventStopFire)

(event EventShootOnce
  (if (>= (- (Utilities|Time|GetTimeSeconds) (Variables|Default|GetLastShootTime)) (Variables|Default|GetShootAniTime))
    (Game|SpawnActorfromClass "/Game/Assets/Blueprints/Bullet.Bullet_C" (Transformation|GetWorldTransform (Variables|Default|Getmazzle)) "Undefined" 0 0)
    (Animation|PlayAnimMontage (Variables|Default|GetGunOwner) "/Game/Assets/Blueprints/Anim/FppLaunMage.FppLaunMage" 1.0 "None")
    (Variables|Default|SetLastShootTime (Utilities|Time|GetTimeSeconds))))

(fn ConstructionScript)