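; First-person shooter player Blueprint that handles movement, look, firing and switching between guns.
; On BeginPlay it creates a rifle and a launcher, shows the gun at index 1, and delegates fire and stop to the current gun.
; Q cycles guns by toggling visibility and plays an equip montage, with a timestamp cooldown blocking firing and re-switching, though not the montage.
; GetAimInfo supplies aim endpoints from two camera-related components.
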(event EventBeginPlay
  (CallFunction|CreatGun "/Game/Assets/Blueprints/Rifle.Rifle_C")
  (CallFunction|CreatGun "/Game/Assets/Blueprints/Launcher.Launcher_C")
  (Variables|Default|SetGunIndex 1)
  (Rendering|SetActorHiddenInGame (CallFunction|GetCurGun) false))

(event Collision|EventActorBeginOverlap
  (params (OtherActor :type Actor%20Object%20Reference)))

(event EventTick
  (params (DeltaSeconds :type Float%20%28single-precision%29)))

(event Input|ActionEvents|InputActionFire
  (params (Key :type Key%20Structure))
  (:Pressed
    (CallFunction|Fire))
  (:Released
    (CallFunction|StopFire)))

(event Input|AxisEvents|InputAxisMove_forward
  (params (AxisValue :type Float%20%28single-precision%29))
  (Pawn|Input|AddMovementInput (Math|Vector|GetForwardVector (Pawn|GetControlRotation :!class /Script/Engine.Pawn)) AxisValue false))

(event Input|AxisEvents|InputAxisTurn
  (params (AxisValue :type Float%20%28single-precision%29))
  (Pawn|Input|AddControllerYawInput AxisValue))

(event Input|AxisEvents|InputAxisLook
  (params (AxisValue :type Float%20%28single-precision%29))
  (Pawn|Input|AddControllerPitchInput AxisValue))

(event Input|AxisEvents|InputAxisMove_Right
  (params (AxisValue :type Float%20%28single-precision%29))
  (Pawn|Input|AddMovementInput (Math|Vector|GetRightVector (Pawn|GetControlRotation :!class /Script/Engine.Pawn)) AxisValue false))

(event Input|KeyboardEvents|Q
  (params (Key :type Key%20Structure))
  (:Pressed
    (CallFunction|SwitchWeapon)
    (Animation|PlayAnimMontage "/Game/Assets/Blueprints/Anim/FppEquip.FppEquip" 1.0 "None")))

(fn ConstructionScript)

(fn Fire
  (if (not (CallFunction|IsSwitching))
    (Default|Fire (CallFunction|GetCurGun))))

(fn StopFire
  (Default|StopFire (CallFunction|GetCurGun)))

(fn SwitchWeapon
  (bind _currentgun (CallFunction|GetCurGun))
  (if (not (CallFunction|IsSwitching))
    (Default|StopFire _currentgun)
    (Rendering|SetActorHiddenInGame _currentgun true)
    (Variables|Default|SetGunIndex (Math|Integer|%(Integer) (+ (Variables|Default|GetGunIndex) 1) (Utilities|Array|Length (Variables|Default|GetGuns))))
    (Rendering|SetActorHiddenInGame (CallFunction|GetCurGun) false)
    (Variables|Default|SetSwitchWeponTime (Utilities|Time|GetTimeSeconds))))

(fn IsSwitching
  (return (< (- (Utilities|Time|GetTimeSeconds) (Variables|Default|GetSwitchWeponTime)) (Variables|Default|GetSwitchTimeLength))))

(fn GetAimInfo
  (return (Transformation|GetWorldLocation (Variables|Default|GetCamera)) (Transformation|GetWorldLocation (Variables|Default|GetCameraAim))))