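; Robot shooter Blueprint that fires its current gun and supplies that gun's aim line.
; GetAimInfo returns the gun arrow's location as start and its normalized forward vector times a fixed range as end, without adding the start.
; AlwaysShoot fires the gun, OnDieOver destroys the actor, and construction makes the mesh block Visibility.
; The rifle creation and unhide logic in the event graph is disconnected and never runs.
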(event EventBeginPlay)

(event Collision|EventActorBeginOverlap
  (params (OtherActor :type Actor%20Object%20Reference)))

(event EventTick
  (params (DeltaSeconds :type Float%20%28single-precision%29)))

(fn ConstructionScript
  (Collision|SetCollisionResponsetoChannel (Variables|Character|GetMesh) "ECC_Visibility" "ECR_Block"))

(fn OnDieOver
  (Actor|DestroyActor))

(fn GetAimInfo
  (bind _currentgun (CallFunction|GetCurGun))
  (bind _arrow (Variables|/Game/Assets/Blueprints/Gun.Gun_C|Getarrow _currentgun))
  (return (Transformation|GetWorldLocation _arrow) (* (Math|Vector|Normalize (Math|Vector|GetForwardVector _arrow)) 3000)))

(fn AlwaysShoot
  (Default|Fire (CallFunction|GetCurGun)))