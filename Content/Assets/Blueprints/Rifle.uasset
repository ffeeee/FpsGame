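; Rifle weapon that gives its owner automatic hitscan fire against Shooter targets.
; Fire plays a montage, attaches a muzzle flash and starts a looping ShootOnce timer, all of which StopFire ends.
; ShootOnce traces along the owner's aim to find a target point, then from the muzzle arrow toward it to apply damage.
; The muzzle trace leaves persistent debug lines, and hits print the target's health.
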(event EventBeginPlay
  (|CallParentFunction) ; This node is disabled and will not be called.\nDrag off pins to build functionality.
)

(event Collision|EventActorBeginOverlap
  (params (OtherActor :type Actor%20Object%20Reference))
  (|CallParentFunction OtherActor) ; This node is disabled and will not be called.\nDrag off pins to build functionality.
)

(event EventTick
  (params (DeltaSeconds :type Float%20%28single-precision%29))
  (|CallParentFunction DeltaSeconds) ; This node is disabled and will not be called.\nDrag off pins to build functionality.
)

(event EventFire
  (Utilities|FlowControl|Sequence
    (:then_0
      (Animation|PlayAnimMontage (Variables|Default|GetGunOwner) "/Game/Assets/Blueprints/Anim/FppRifleMotage.FppRifleMotage" 1.0 "None")
      (bind _returnvalue (Effects|SpawnEmitterAttached "/Game/Assets/Effects/ParticleSystems/Weapons/AssaultRifle/Muzzle/P_AssaultRifle_MF.P_AssaultRifle_MF" (Variables|Default|Getarrow) "None"))
      (Variables|Default|SetFireParticle _returnvalue))
    (:then_1
      (CallFunction|ShootOnce)
      (Utilities|Time|SetTimerbyFunctionName 0 "ShootOnce" 0.15 true))
    (:then_2
      (Variables|Default|SetIsFire true))))

(event EventShootOnce
  (bind _gunowner (Variables|Default|GetGunOwner))
  (bind (_aimstartpoint _aimendpoint) (Default|GetAimInfo _gunowner))
  (Utilities|FlowControl|Sequence
    (:then_0
      (bind (_outhit _returnvalue) (Collision|LineTraceByChannel _aimstartpoint _aimendpoint "TraceTypeQuery1" false 0 "None"))
      (if _returnvalue
        (Variables|Default|SetCameraAimPos (.Location (Collision|BreakHitResult _outhit)))
        (else
          (Variables|Default|SetCameraAimPos _aimendpoint))))
    (:then_1
      (bind (_outhit_2 _returnvalue_2) (Collision|LineTraceByChannel (Transformation|GetWorldLocation (Variables|Default|Getarrow)) (Variables|Default|GetCameraAimPos) "TraceTypeQuery1" false 0 "Persistent"))
      (if _returnvalue_2
        (bind _asshooter (Utilities|Casting|CastToShooter (.HitActor (Collision|BreakHitResult _outhit_2))))
        (Default|TakeDamage _asshooter 1e+01)
        (Development|PrintString (Utilities|String|ToString(Float) (Variables|/Game/Assets/Blueprints/Shooter.Shooter_C|GetHealth _asshooter)))))))

(event EventStopFire
  (if (Variables|Default|GetIsFire)
    (Utilities|FlowControl|Sequence
      (:then_0
        (Animation|StopAnimMontage (Variables|Default|GetGunOwner) "/Game/Assets/Blueprints/Anim/FppRifleMotage.FppRifleMotage")
        (Components|DestroyComponent (Variables|Default|GetFireParticle))
        (Variables|Default|SetIsFire false))
      (:then_1
        (Utilities|Time|ClearTimerbyFunctionName 0 "ShootOnce")))))

(fn ConstructionScript
  (|CallParentFunction))