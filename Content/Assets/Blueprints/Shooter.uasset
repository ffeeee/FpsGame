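; Base shooter character blueprint that manages health, death and a set of carried guns.
; TakeDamage subtracts and prints health, then on death detaches the controller and schedules OndieOver, which is not defined here.
; CreatGun spawns hidden guns on the RightWeapon socket, sets their owner and stores them for GetCurGun's index lookup and cleanup on Destroyed.
; GetAimInfo returns only zero vectors.
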(event EventBeginPlay)

(event Collision|EventActorBeginOverlap
  (params (OtherActor :type Actor%20Object%20Reference)))

(event EventTick
  (params (DeltaSeconds :type Float%20%28single-precision%29)))

(event EventDestroyed
  (for _array_element (Variables|Default|GetGuns)
    (Actor|DestroyActor _array_element)))

(fn ConstructionScript)

(fn TakeDamage
  (params (Damage :type Float%20%28single-precision%29))
  (bind _output_get (Variables|Default|SetHealth (- (Variables|Default|GetHealth) Damage)))
  (Development|PrintString (Utilities|String|ToString(Float) _output_get))
  (if (CallFunction|IsDead)
    (Class|Pawn|DetachfromControllerPendingDestroy)
    (Utilities|Time|SetTimerbyFunctionName 0 "OndieOver" 5.0)))

(fn IsDead
  (return (<= (Variables|Default|GetHealth) 0.0)))

(fn GetAimInfo
  (return "0, 0, 0" "0, 0, 0"))

(fn CreatGun
  (params (Gun :type Gun%20Class%20Reference))
  (bind _returnvalue (Game|SpawnActorfromClass Gun (Math|Transform|MakeTransform "0, 0, 0" "0, 0, 0" "1,1,1") "Undefined" 0 0))
  (Transformation|AttachComponentToComponent _returnvalue (Variables|Character|GetMesh) "RightWeapon" "SnapToTarget" "SnapToTarget" "SnapToTarget" true)
  (Variables|/Game/Assets/Blueprints/Gun.Gun_C|SetGunOwner _returnvalue self)
  (Utilities|Array|Add (Variables|Default|GetGuns) _returnvalue)
  (Rendering|SetActorHiddenInGame _returnvalue true))

(fn GetCurGun
  (return (Utilities|Array|Get(acopy) (Variables|Default|GetGuns) (Variables|Default|GetGunIndex))))