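; AI controller that drives a robot enemy to chase the player while shooting.
; Shortly after BeginPlay it casts the controlled pawn to RobotShooter and calls AlwaysShoot once.
; It then issues AIMoveTo toward the first player's pawn with an acceptance radius, reissuing the move every second through a delayed loop instead of using Tick.
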(event EventBeginPlay
  (Utilities|FlowControl|Delay 0.2)
  (Default|AlwaysShoot (CallFunction|GetRobotShoot))
  (AI|AIMoveTo (Pawn|GetControlledPawn) "0, 0, 0" (Game|Player|GetPlayerPawn 0) 2e+02 false :!label _label
    (:then
      (Utilities|FlowControl|Delay 1.0)
      (goto _label))))

(event EventTick
  (params (DeltaSeconds :type Float%20%28single-precision%29)))

(fn ConstructionScript)

(fn GetRobotShoot
  (bind _asrobot_shooter (Utilities|Casting|CastToRobotShooter (Pawn|GetControlledPawn)))
  (return _asrobot_shooter))